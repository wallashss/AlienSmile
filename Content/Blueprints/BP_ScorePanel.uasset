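; BP_ScorePanel is a score display that shows an integer score through its Score text component.
; It hides Score on BeginPlay until OnInitScore sets the first value and makes it visible.
; OnScoreUpdate refreshes the number through the same UpdateScore function, which converts the integer to text, without changing visibility.
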(event `self.ReceiveBeginPlay`
  ;[1 1 1] Initialize. Set Objects Invisible
  (`SceneComponent.SetVisibility` (`self.Score`) false true)
  (`KismetSystemLibrary.PrintString` "Set invisble"))

(event `self.OnScoreUpdate`
  (params (Score :type Integer))
  (`self.UpdateScore` Score))

(event `self.OnInitScore`
  (params (Score :type Integer))
  (`self.UpdateScore` Score)
  (`SceneComponent.SetVisibility` (`self.Score`) true true)
  (`KismetSystemLibrary.PrintString` "Score Inited"))

(fn `UpdateScore`
  (params (Score :type Integer))
  (`Text3DComponent.SetText` (`self.Score`) (`KismetTextLibrary.Conv_IntToText` Score)))

(fn `UserConstructionScript`)
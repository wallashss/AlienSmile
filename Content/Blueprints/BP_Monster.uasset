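; BP_Monster is the alien monster enemy, handling its animation and sound reactions to smiling, damage, death and winning.
; Monster state events swap looping walk, smile and victory animations or a one-shot death animation, with a laugh on smiling and a punch sound on damage.
; A mouth sphere collider calls SetDamage when a Projectile overlaps it; damage logic is not defined in this graph.
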(event `self.OnMonsterWinner`
  ;[1 1 1] Monster WINS
  (`SkeletalMeshComponent.PlayAnimation` (`self.Mesh`) "/Game/Characters/AlienFinal/Alien/Alien_Anim_GR_Vitória.Alien_Anim_GR_Vitória" true))

(event `self.MouthSphereCollider.OnComponentBeginOverlap`
  (params (OverlappedComponent :type "PrimitiveComponent Object Reference") (OtherActor :type "Actor Object Reference") (OtherComp :type "PrimitiveComponent Object Reference") (OtherBodyIndex :type Integer) (bFromSweep :type Boolean) (SweepResult :type "HitResult Structure (by ref)"))
  ;[1 1 1] Test Collision with Projectile
  (cast `/Game/VRTemplate/Blueprints/Projectile` OtherActor)
  (`KismetSystemLibrary.PrintString` "YES")
  (`self.SetDamage`))

(event `self.OnMonsterSmiling`
  ;[1 1 1] Smile
  (`SkeletalMeshComponent.PlayAnimation` (`self.Mesh`) "/Game/Characters/AlienFinal/Alien/Alien_Anim_GR_Sorrindo.Alien_Anim_GR_Sorrindo" true)
  (`GameplayStatics.PlaySound2D` "/Game/Sound/341736__scorpion67890__flail-demon-laugh.341736__scorpion67890__flail-demon-laugh" 1.0 1.0 0.0 null null))

(event `self.OnMonsterStopSmiling`
  ;[1 1 1] Stop Smile
  (`SkeletalMeshComponent.PlayAnimation` (`self.Mesh`) "/Game/Characters/AlienFinal/Alien/Alien_Anim_GR_Andando.Alien_Anim_GR_Andando" true))

(event `self.OnMonsterDamage`
  ;[1 1 1] Damage
  (`GameplayStatics.PlaySoundAtLocation` "/Game/Sound/qubodupPunch05.qubodupPunch05" (`self.K2_GetActorLocation`) (struct) 1.0 1.0 0.0 null null null null)
  (`KismetSystemLibrary.PrintString` "DAMAGe"))

(event `self.OnMonsterDead`
  (`SkeletalMeshComponent.PlayAnimation` (`self.Mesh`) "/Game/Characters/AlienFinal/Alien/Alien_Anim_GR_Morrendo.Alien_Anim_GR_Morrendo" false))

(fn `UserConstructionScript`)
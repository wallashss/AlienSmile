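; BP_Monkey is a grabbable monkey item that plays a cymbal sound and animates when picked up.
; On grab, if no sound is valid, it spawns the cymbal audio attached to the skeletal mesh and starts a looping animation.
; On drop, it lowers that sound's volume, then stops it after a short delay, while the animation is left looping.
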(event `self.GrabComponent.OnGrabbed`
  (`/Engine/EditorBlueprintResources/StandardMacros.IsValid` (`self.Sound`)
    (:`Is Not Valid`
      (bind _returnvalue (`GameplayStatics.SpawnSoundAttached` "/Game/Sound/317083__shpira__cymbal-second1_edited.317083__shpira__cymbal-second1_edited" (`self.SkeletalMesh`) "None" (0.0 0.0 0.0) (struct) "KeepRelativeOffset" false 1.0 1.0 0.0 null null))
      (set `self.Sound` _returnvalue)
      (`SkeletalMeshComponent.PlayAnimation` (`self.SkeletalMesh`) "/Game/Characters/Itens/JollyChimp4/Monkey_Anim.Monkey_Anim" true))))

(event `self.GrabComponent.OnDropped`
  (bind _sound (`self.Sound`))
  (`/Engine/EditorBlueprintResources/StandardMacros.IsValid` _sound
    (:`Is Valid`
      (`AudioComponent.SetVolumeMultiplier` _sound 0.3)
      (`KismetSystemLibrary.Delay` 2.0)
      (`AudioComponent.Stop` (`self.Sound`)))))

(fn `UserConstructionScript`)
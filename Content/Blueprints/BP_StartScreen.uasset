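; BP_StartScreen is a grabbable start object that shows tutorial prompts and starts the game once dropped.
; It binds to GrabComponent's grab and drop events, enabling simulate-on-drop and switching the visible instruction from MiddleTutorial to Shoot to WellDone.
; Each interaction plays a rubber chicken sound.
; After the drop, a short delay precedes InitGame on AlienGameState, then the actor destroys itself.
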(event `self.ReceiveBeginPlay`
  (add `/Game/VRTemplate/Blueprints/GrabComponent.OnGrabbed` (`self.GrabComponent`) (delegate `OnStartObjGrabbed`))
  (add `/Game/VRTemplate/Blueprints/GrabComponent.OnDropped` (`self.GrabComponent`) (delegate `OnStartObjDropped`)))

(event `OnStartObjGrabbed`
  ;[1 1 1] Activate simulation when it is released
  (set `/Game/VRTemplate/Blueprints/GrabComponent.bSimulateOnDrop` true (`self.GrabComponent`))
  ;[1 1 1] Update instuctions
  (`SceneComponent.SetVisibility` (`self.Middle Tutorial`) false false)
  (`SceneComponent.SetVisibility` (`self.Shoot`) false false)
  (`SceneComponent.SetVisibility` (`self.Shoot`) true false)
  (`GameplayStatics.PlaySoundAtLocation` "/Game/Sound/628157__rufusmack__rubberchicken_cliped.628157__rufusmack__rubberchicken_cliped" (`self.K2_GetActorLocation`) (struct) 1.0 1.0 0.0 null null null null))

(event `OnStartObjDropped`
  ;[1 1 1] Update instructions
  (`GameplayStatics.PlaySoundAtLocation` "/Game/Sound/628157__rufusmack__rubberchicken_cliped2.628157__rufusmack__rubberchicken_cliped2" (`self.K2_GetActorLocation`) (struct) 1.0 1.0 0.0 null null null null)
  (`SceneComponent.SetVisibility` (`self.Shoot`) false false)
  (`SceneComponent.SetVisibility` (`self.WellDone`) true false)
  ;[1 1 1] init game
  (bind _asalien_game_state (cast `AlienGameState` (`GameplayStatics.GetGameState`)))
  (`KismetSystemLibrary.Delay` 3.0)
  (`AlienGameState.InitGame` _asalien_game_state)
  (`self.K2_DestroyActor`))

(fn `UserConstructionScript`)